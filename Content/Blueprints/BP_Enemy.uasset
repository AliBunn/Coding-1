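; BP_Enemy is an enemy actor that dies when its capsule overlaps the third-person player character or a BP_Crate.
; Either overlap sets Health below zero and prints a hit message.
; From BeginPlay, CheckHealth polls Health by re-calling itself after a short delay, forming a timed loop without Tick, and destroys the actor once Health is negative.
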(event `self.ReceiveBeginPlay`
  (`self.Check Health`) ; while true loop
)

(event `Check Health`
  (`KismetSystemLibrary.Delay` 0.2)
  (if (>= (`self.Health`) 0.0)
    (`self.Check Health`) ; call function
    (else
      (`self.K2_DestroyActor`))))

(event `self.Capsule.OnComponentBeginOverlap`
  (params (OverlappedComponent :type "PrimitiveComponent Object Reference") (OtherActor :type "Actor Object Reference") (OtherComp :type "PrimitiveComponent Object Reference") (OtherBodyIndex :type Integer) (bFromSweep :type Boolean) (SweepResult :type "HitResult Structure (by ref)"))
  (cast `/Game/ThirdPerson/Blueprints/BP_ThirdPersonCharacter` OtherActor
    (:`then`
      _)
    (:`CastFailed`
      (cast `/Game/Blueprints/BP_Crate` OtherActor)))
  (set `self.Health` -1.0)
  (`KismetSystemLibrary.PrintString` "I hit!" true true (struct :`R` 1.0 :`G` 0.096025 :`B` 0.555027 :`A` 1.0)))

(fn `UserConstructionScript`)