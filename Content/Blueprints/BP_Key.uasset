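; BP_Key is a key pickup that adds to the player's TotalKeys count when hit.
; A Sphere component hit casts the other actor to BP_ThirdPersonCharacter, increments its TotalKeys, then destroys the key.
; It prints the new total before capping it at 10, so the message can show an uncapped value.
; A disconnected node that resets TotalKeys to zero never runs.
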(event `self.Sphere.OnComponentHit`
  (params (HitComponent :type "PrimitiveComponent Object Reference") (OtherActor :type "Actor Object Reference") (OtherComp :type "PrimitiveComponent Object Reference") (NormalImpulse :type "Vector Structure") (Hit :type "HitResult Structure (by ref)"))
  (bind _asbp_third_person_character (cast `/Game/ThirdPerson/Blueprints/BP_ThirdPersonCharacter` OtherActor)) ; Was it the player that ran into us?
  (bind _totalkeys (`/Game/ThirdPerson/Blueprints/BP_ThirdPersonCharacter.TotalKeys` _asbp_third_person_character))
  (`/Engine/EditorBlueprintResources/StandardMacros.IncrementInt` _totalkeys
    (:`  `
      (`self.K2_DestroyActor`)
      (`KismetSystemLibrary.PrintString` (`KismetStringLibrary.Concat_StrStr` "TotalKeys =" (`KismetStringLibrary.Conv_IntToString` _totalkeys)))
      (if (> _totalkeys 10)
        (set `/Game/ThirdPerson/Blueprints/BP_ThirdPersonCharacter.TotalKeys` 10 _asbp_third_person_character)))))

(fn `UserConstructionScript`)