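; BP_Item is an item Blueprint that rolls its stats at BeginPlay and automatically damages an enemy.
; Constructor sets Damage by Type, with weapons rolling random damage and taking a shuffled name if unnamed.
; After a debug print and short delay, Attack subtracts Damage as a percentage from the BP_Enemy found in the level.
; A Timeline also raises the Cube mesh, and a separate event hides it.
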(event `hide startend`
  (`SceneComponent.SetVisibility` (`self.Cube`) false false))

(event `self.ReceiveBeginPlay`
  (`|ExecutionSequence`
    (:`then_0`
      (`self.Constructor`)
      (`KismetSystemLibrary.PrintString` (`KismetStringLibrary.Concat_StrStr` "Name:" (`self.Name`) "Damage:" (`KismetStringLibrary.Conv_IntToString` (`self.Damage`))) true true (struct :`R` 0.419974 :`B` 1.0 :`A` 1.0) 8.0)
      (`KismetSystemLibrary.Delay` 0.2)
      (bind _returnvalue (`GameplayStatics.GetActorOfClass` "/Game/Blueprints/BP_Enemy.BP_Enemy_C"))
      (`self.Attack` _returnvalue))
    (:`then_1`
      (bind (_direction _newtrack_0) (`Timeline|Timeline`)
        (:`Update`
          (`SceneComponent.K2_SetRelativeLocation` (`self.Cube`) (`KismetMathLibrary.MakeVector` 0.0 0.0 (`KismetMathLibrary.Lerp` 0.0 100.0 _newtrack_0)) false false)
          (`KismetSystemLibrary.PrintString` "Hello"))))))

(fn `Attack`
  (params (GivenEnemy :type "/Game/Blueprints/BP_Enemy Object Reference"))
  (set `/Game/Blueprints/BP_Enemy.Health` (- (`/Game/Blueprints/BP_Enemy.Health` GivenEnemy) (* (`KismetMathLibrary.Conv_IntToDouble` (`self.Damage`)) 0.01)) GivenEnemy) ; set health
)

(fn `Constructor`
  (bind _weaponnames (`self.WeaponNames`))
  (switch `/Game/Classes/ItemType` (`self.Type`)
    (:`NewEnumerator0`
      (set `self.Damage` (`KismetMathLibrary.RandomIntegerInRange` 3 6))
      (if (`KismetStringLibrary.EqualEqual_StrStr` (`self.Name`))
        (`KismetArrayLibrary.Array_Shuffle` _weaponnames)
        (set `self.Name` (`|GetArrayItem` _weaponnames))))
    (:`NewEnumerator1`
      (set `self.Damage` 1))
    (:`NewEnumerator2`
      (set `self.Damage` 0))))

(fn `UserConstructionScript`)